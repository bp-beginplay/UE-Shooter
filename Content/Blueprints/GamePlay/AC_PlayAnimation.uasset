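; AC_PlayAnimation is a component that plays the animation of its owning Skeletal Mesh Actor when its Action event fires.
; Action casts the owner to SkeletalMeshActor and plays its skeletal mesh component without looping.
; With the FlipFlop option enabled, each call first alternates the play rate between forward and reverse, so the animation works as a toggle.
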(event EventBeginPlay
  (|CallParentFunction) ; This node is disabled and will not be called.\nDrag off pins to build functionality.
)

(event EventAction
  (params (Owner :type Pawn%20Object%20Reference))
  (bind _as스켈레탈_메시_액터 (Utilities|Casting|CastToSkeletalMeshActor (Components|GetOwner)))
  (if (Variables|Default|GetFlipFlop)
    (bind _isa (Utilities|FlowControl|FlipFlop)
      (:A
        _)
      (:B
        _))
    (Components|Timeline|SetPlayRate (Variables|/Script/Engine.SkeletalMeshActor|GetSkeletalMeshComponent _as스켈레탈_메시_액터) (select _isa 1.0 -1.0))
    (Audio|Components|Audio|Play (Variables|/Script/Engine.SkeletalMeshActor|GetSkeletalMeshComponent _as스켈레탈_메시_액터) false)
    (else
      (Audio|Components|Audio|Play (Variables|/Script/Engine.SkeletalMeshActor|GetSkeletalMeshComponent _as스켈레탈_메시_액터) false))))