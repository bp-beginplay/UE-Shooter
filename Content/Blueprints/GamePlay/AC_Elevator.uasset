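; AC_Elevator is a component that drives an elevator through the animation on its owning Skeletal Mesh Actor.
; On BeginPlay it stops the mesh's single-node animation and turns looping off.
; Each Action event flips between a slow forward and a slow reverse play rate, then plays without looping, so one clip serves both directions of travel.
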(event EventBeginPlay
  (|CallParentFunction)
  (bind _as스켈레탈_메시_액터 (Utilities|Casting|CastToSkeletalMeshActor (Components|GetOwner)))
  (bind _as애님_단일_노드_인스턴스 (Utilities|Casting|CastToAnimSingleNodeInstance (Components|SkeletalMesh|GetAnimInstance (Variables|/Script/Engine.SkeletalMeshActor|GetSkeletalMeshComponent _as스켈레탈_메시_액터))))
  (Components|Timeline|SetLooping _as애님_단일_노드_인스턴스 false)
  (Class|AnimSingleNodeInstance|SetPlaying _as애님_단일_노드_인스턴스 false))

(event EventAction
  (params (Owner :type Pawn%20Object%20Reference))
  (bind _as스켈레탈_메시_액터 (Utilities|Casting|CastToSkeletalMeshActor (Components|GetOwner)))
  (Utilities|FlowControl|FlipFlop
    (:A
      (Components|Timeline|SetPlayRate (Variables|/Script/Engine.SkeletalMeshActor|GetSkeletalMeshComponent _as스켈레탈_메시_액터) 0.2))
    (:B
      (Components|Timeline|SetPlayRate (Variables|/Script/Engine.SkeletalMeshActor|GetSkeletalMeshComponent _as스켈레탈_메시_액터) -0.2)))
  (Audio|Components|Audio|Play (Variables|/Script/Engine.SkeletalMeshActor|GetSkeletalMeshComponent _as스켈레탈_메시_액터) false))